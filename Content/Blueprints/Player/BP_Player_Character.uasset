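; Player character Blueprint for first-person play, handling movement, look, jump and weapon fire input.
; On possession, the authority creates an auto rifle through BPWeaponsManager and selects it as the current weapon.
; Fire input routes through the ServerFire event to the current weapon's UseWeapon.
; GetVissibleMesh returns the hands mesh when locally controlled and the body mesh otherwise.
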(event `self.ReceivePossessed`
  (params (NewController :type "Controller Object Reference"))
  (`/Engine/EditorBlueprintResources/ActorMacros.Switch Has Authority`
    (:`Authority`
      (bind _weapon (`/Game/Blueprints/Components/Player/BP_WeaponsManager.CreateWeapon` (`self.BP_WeaponsManager`) "/Game/Blueprints/Weapons/BP_Weapon_AutoRifles.BP_Weapon_AutoRifles_C"))
      (`/Game/Blueprints/Components/Player/BP_WeaponsManager.SelectWeapon` (`self.BP_WeaponsManager`) _weapon))))

(event `InputAction|Fire`
  (params (Key :type "Key Structure"))
  (:`Pressed`
    (`self.ServerFire`)))

(event `ServerFire`
  (`/Game/Blueprints/Weapons/BP_Weapon.UseWeapon` (`/Game/Blueprints/Components/Player/BP_WeaponsManager.CurrentWeapon` (`self.BP_WeaponsManager`))))

(event `InputAxis|LookUp`
  (params (AxisValue :type "Float (single-precision)"))
  (`self.AddControllerPitchInput` AxisValue))

(event `InputAxis|MoveForward`
  (params (AxisValue :type "Float (single-precision)"))
  (`self.AddMovementInput` (`self.GetActorForwardVector`) AxisValue))

(event `InputAxis|Turn`
  (params (AxisValue :type "Float (single-precision)"))
  (`self.AddControllerYawInput` AxisValue))

(event `InputAction|Jump`
  (params (Key :type "Key Structure"))
  (:`Pressed`
    (`self.Jump`)))

(event `InputAxis|MoveRight`
  (params (AxisValue :type "Float (single-precision)"))
  (`self.AddMovementInput` (`self.GetActorRightVector`) AxisValue))

(fn `GetVissibleMesh`
  (returns (SkeletalMesh :type "SkeletalMeshComponent Object Reference"))
  (return (select `bool` (`self.IsLocallyControlled`) :`false` (`self.Mesh`) :`true` (`self.Hands Mesh`))))

(fn `UserConstructionScript`)