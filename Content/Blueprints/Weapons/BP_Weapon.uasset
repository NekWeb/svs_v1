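; BP_Weapon is a weapon actor that handles ammo and fire-rate gating, with no projectile, damage or effect logic.
; UseWeapon checks for ammo and no active cooldown, spends a round, starts a UseRite-second timer and returns whether it fired.
; StopRateDelay clears the cooldown and, with AutoFire, calls UseWeapon again until ammo runs out.
; StopUseWeapon is empty and FireActive is never read, so nothing here interrupts automatic fire.
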(fn `AbleToUseWeapon`
  (returns (Out :type Boolean))
  (return (and (> (`self.CurrentAmmo`) 0) (not (`self.UseFreezeByRate`)))))

(fn `StopRateDelay`
  (set `self.UseFreezeByRate` false)
  (if (`self.AutoFire`)
    (`self.UseWeapon`)))

(fn `StopUseWeapon`)

(fn `UserConstructionScript`)

(fn `UseWeapon`
  (returns (Used :type Boolean))
  (if (`self.AbleToUseWeapon`)
    (`/Engine/EditorBlueprintResources/StandardMacros.DecrementInt` (`self.CurrentAmmo`)
      (:`  `
        (`KismetSystemLibrary.K2_SetTimer` null "StopRateDelay" (`self.UseRite`))
        (set `self.UseFreezeByRate` true)
        (if (`self.AutoFire`)
          (set `self.FireActive` true))
        (return true)))
    (else
      (set `self.FireActive` false)
      (return false))))